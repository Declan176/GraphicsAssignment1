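; Door Blueprint that slides open when enough pressure switches are active.
; Activation and deactivation events adjust an active-switch count and compare it to the required number.
; Meeting the threshold plays the Door_open timeline, otherwise it reverses.
; The timeline moves the door along relative X, keeping Y and Z at fixed offsets.
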(event Custom|Switchactivated
  (Math|Integer|IncrementInt (Variables|Default|Getpressure%20switched%20active)
    (:%20%20
      (if (>= (Variables|Default|Getpressure%20switched%20active) (Variables|Default|Getpressure%20switches%20needed))
        (bind _dor_position (Timeline|door_open Play)
          (:Update
            (Transformation|SetRelativeLocation (Variables|Default|Getdoor) (Math|Vector|MakeVector _dor_position 3e+01 1.1e+02) false false)))
        (else
          (Timeline|door_open Reverse))))))

(event Custom|SwitchDeactivated
  (Math|Integer|DecrementInt (Variables|Default|Getpressure%20switched%20active)
    (:%20%20
      (if (>= (Variables|Default|Getpressure%20switched%20active) (Variables|Default|Getpressure%20switches%20needed))
        (bind _dor_position (Timeline|door_open Play)
          (:Update
            (Transformation|SetRelativeLocation (Variables|Default|Getdoor) (Math|Vector|MakeVector _dor_position 3e+01 1.1e+02) false false)))
        (else
          (Timeline|door_open Reverse))))))

(fn ConstructionScript)